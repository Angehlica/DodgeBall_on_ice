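; Moveable obstacle actor that drops its DropObstacle component after it has been overlapped enough times.
; Each actor begin-overlap increments a hit counter, with no filter on the overlapping actor since the branch condition is a constant true.
; Once the count reaches the threshold, the DropObject event enables physics simulation on the component, and later overlaps call it again.
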(event `self.ReceiveActorBeginOverlap`
  (params (OtherActor :type "Actor Object Reference"))
  (if true
    (set `self.HitCounted` (+ 1 (`self.HitCounted`)))
    (if (>= (`self.HitCounted`) 3)
      (`self.DropObject`))))

(event `DropObject`
  (`PrimitiveComponent.SetSimulatePhysics` (`self.Drop_obstacle`) true))

(fn `UserConstructionScript`)