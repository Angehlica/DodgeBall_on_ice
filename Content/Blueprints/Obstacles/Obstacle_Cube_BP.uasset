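; Obstacle cube Blueprint that moves along the world X axis, centred on its placed location.
; On BeginPlay it stores its location, then a timeline lerps X between fixed offsets either side of that point, keeping current Y and Z, without sweep.
; Two other timeline movers, a Y-axis lerp and an additive offset, are left unconnected and never run.
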(event `self.ReceiveBeginPlay`
  (bind _x (.x (`self.Positions`)))
  (set `self.Positions` (`self.K2_GetActorLocation`))
  (bind (_direction _newtrack_3) (`Timeline|Timeline_2` :!via `PlayFromStart`)
    (:`Update`
      (`self.K2_SetActorLocation` (`KismetMathLibrary.MakeVector` (`KismetMathLibrary.Lerp` (- _x 1000.0) (+ _x 1000.0) _newtrack_3) (.y (`self.K2_GetActorLocation`)) (.z (`self.K2_GetActorLocation`)))))))

(fn `UserConstructionScript`)