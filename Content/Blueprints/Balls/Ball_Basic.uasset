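; Basic dodgeball actor that tracks its owner and whether it can be picked up.
; Overlapping a Floor-tagged actor clears the owner, re-enables pickup, restores the default outline and stops the trail.
; Respawn does the same, also zeroing velocity and returning the ball to its start location.
; SetMaterial tints a dynamic material's outline and the trail emitter by color, with black outline as default.
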(event `self.ReceiveBeginPlay`
  ;[1 1 1] Begin Play / Set Start Location
  (set `self.StartLocation` (`self.K2_GetActorLocation`))
  ;[1 1 1] Skapa Dynamiskt material för att kundra ändra paramtetrar i runtime
  (bind _returnvalue (`PrimitiveComponent.CreateDynamicMaterialInstance` (`self.Sphere`) 0 null))
  (set `self.DynamicMaterialRef` _returnvalue))

(event `Respawn`
  ;[1 1 1] Out Of Bounds Respawn (triggered By Level BP)
  (`PrimitiveComponent.SetPhysicsLinearVelocity` (`self.Sphere`) (0.0 0.0 0.0) false "None")
  (set `self.BallOwner` null)
  (set `self.AbleToPickup` true)
  (`self.SetMaterial` "NewEnumerator4")
  (`ActorComponent.SetActive` (`self.TrailEmitter`) false false)
  (`self.K2_SetActorLocation` (`self.StartLocation`)))

(event `self.CollisionSphere.OnComponentBeginOverlap`
  (params (OverlappedComponent :type "PrimitiveComponent Object Reference") (OtherActor :type "Actor Object Reference") (OtherComp :type "PrimitiveComponent Object Reference") (OtherBodyIndex :type Integer) (bFromSweep :type Boolean) (SweepResult :type "HitResult Structure (by ref)"))
  ;[1 1 1] On Hit generation call hit event in player / print if object then enable pickup
  (cast `/Game/Blueprints/Characters/DodgeCharacter` OtherActor
    (:`CastFailed`
      (if (`self.ActorHasTag` OtherActor "Floor")
        (set `self.BallOwner` null)
        (set `self.AbleToPickup` true)
        (`self.SetMaterial` "NewEnumerator4")
        (`ActorComponent.SetActive` (`self.TrailEmitter`) false false)))))

(event `SetMaterial`
  (params (NewParam :type "/Game/Blueprints/Characters/enum_PlayerColor Enum" :default "NewEnumerator0"))
  (bind _dynamicmaterialref (`self.DynamicMaterialRef`))
  (bind _trailemitter (`self.TrailEmitter`))
  ;[1 1 1] Ändra OutlineFärg vid kontakt med spelare
  (switch `/Game/Blueprints/Characters/enum_PlayerColor` NewParam
    (:`NewEnumerator0`
      (`MaterialInstanceDynamic.SetVectorParameterValue` _dynamicmaterialref "OutlineColor" (struct :`R` 1.0 :`A` 1.0))
      ;[1 1 1] Ändra färg på trailEmittern
      (`ParticleSystemComponent.SetColorParameter` _trailemitter "TrailColor" (struct :`R` 1.0 :`A` 1.0)))
    (:`NewEnumerator1`
      (`MaterialInstanceDynamic.SetVectorParameterValue` _dynamicmaterialref "OutlineColor" (struct :`B` 1.0 :`A` 1.0))
      (`ParticleSystemComponent.SetColorParameter` _trailemitter "TrailColor" (struct :`B` 1.0 :`A` 1.0)))
    (:`NewEnumerator2`
      (`MaterialInstanceDynamic.SetVectorParameterValue` _dynamicmaterialref "OutlineColor" (struct :`G` 1.0 :`A` 1.0))
      (`ParticleSystemComponent.SetColorParameter` _trailemitter "TrailColor" (struct :`G` 1.0 :`A` 1.0)))
    (:`NewEnumerator3`
      (`MaterialInstanceDynamic.SetVectorParameterValue` _dynamicmaterialref "OutlineColor" (struct :`R` 1.0 :`G` 1.0 :`A` 1.0))
      (`ParticleSystemComponent.SetColorParameter` _trailemitter "TrailColor" (struct :`R` 1.0 :`G` 1.0 :`A` 1.0)))
    (:`NewEnumerator4`
      (`MaterialInstanceDynamic.SetVectorParameterValue` _dynamicmaterialref "OutlineColor" (struct :`A` 1.0)))))

(fn `UserConstructionScript`)