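; Exploding Robot 1 actor that breaks into physics-driven body parts, fades out and destroys itself.
; On BeginPlay it enables physics simulation on every robot mesh piece, then after a short delay plays a timeline driving the FadeRobot1 scalar in the RobotParams1 material parameter collection.
; When the timeline finishes, it sets that shared parameter to 1 before destroying the actor.
; A RadialForce impulse branch exists but is disconnected.
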(event `self.ReceiveBeginPlay`
  (`PrimitiveComponent.SetSimulatePhysics` (`|MakeArray` (`self.SM_Robot_01_LowerArm`) (`self.SM_Robot_01_Arm001`) (`self.SM_Robot_01_Claw003`) (`self.SM_Robot_01_Claw004`) (`self.SM_Robot_01_Claw1`) (`self.SM_Robot_01_Claw2`) (`self.SM_Robot_01_Hand`) (`self.SM_Robot_01_Hand001`) (`self.SM_Robot_01_Leg`) (`self.SM_Robot_01_Leg001`) (`self.SM_Robot_01_Arm`) (`self.SM_Robot_01_LowerArm001`) (`self.SM_Robot_01_LowerLeg`) (`self.SM_Robot_01_LowerLeg001`) (`self.SM_Robot_01_LP`) (`self.SM_Robot_01_LP_Head`) (`self.SM_Robot_01_UpperArm`) (`self.SM_Robot_01_UpperArm001`) (`self.SM_Robot_01_UpperLeg`) (`self.SM_Robot_01_UpperLeg001`) :!type "PrimitiveComponent Object Reference") true)
  (`KismetSystemLibrary.Delay` 0.5)
  (bind (_direction _newtrack_0) (`Timeline|Timeline_0` :!via `PlayFromStart`)
    (:`Update`
      (`KismetMaterialLibrary.SetScalarParameterValue` "/Game/Materials/RobotParams1.RobotParams1" "FadeRobot1" _newtrack_0))
    (:`Finished`
      (`KismetSystemLibrary.Delay` 0.0)
      (`KismetMaterialLibrary.SetScalarParameterValue` "/Game/Materials/RobotParams1.RobotParams1" "FadeRobot1" 1.0)
      (`self.K2_DestroyActor`))))

(fn `UserConstructionScript`)