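; Exploded-robot debris actor for ExploadingRobot2 that scatters the robot's separate mesh parts, fades them and removes itself.
; BeginPlay turns on physics for the parts, then after a short delay a timeline drives the FadeRobot3 scalar in the shared RobotParams3 material parameter collection.
; When the timeline finishes, it sets that global parameter to 1 and destroys the actor.
; The RadialForce impulse branch is disconnected and never runs.
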(event `self.ReceiveBeginPlay`
  (`PrimitiveComponent.SetSimulatePhysics` (`|MakeArray` (`self.SM_Robot_02_Knee`) (`self.SM_Robot_02_Claw005`) (`self.SM_Robot_02_Claw006`) (`self.SM_Robot_02_Claw007`) (`self.SM_Robot_02_Claw008`) (`self.SM_Robot_02_Head`) (`self.SM_Robot_02_Body`) (`self.SM_Robot_02_Knee001`) (`self.SM_Robot_02_Shoulder`) (`self.SM_Robot_02_Shoulder001`) (`self.SM_Robot_02_UpperLeg`) (`self.SM_Robot_02_UpperLeg002`) :!type "PrimitiveComponent Object Reference") true)
  (`KismetSystemLibrary.Delay` 0.5)
  (bind (_direction _newtrack_0) (`Timeline|Timeline_0` :!via `PlayFromStart`)
    (:`Update`
      (`KismetMaterialLibrary.SetScalarParameterValue` "/Game/Materials/RobotParams3.RobotParams3" "FadeRobot3" _newtrack_0))
    (:`Finished`
      (`KismetSystemLibrary.Delay` 0.0)
      (`KismetMaterialLibrary.SetScalarParameterValue` "/Game/Materials/RobotParams3.RobotParams3" "FadeRobot3" 1.0)
      (`self.K2_DestroyActor`))))

(fn `UserConstructionScript`)