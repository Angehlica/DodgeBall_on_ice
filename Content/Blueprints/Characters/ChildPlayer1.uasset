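; Child player character for the red Robot1 in a ball-throwing game, supplying its look and animation hooks.
; The construction script runs the parent's, then sets the player color enum plus red default and glowing invulnerability materials.
; Custom events cast the mesh's anim instance to Robot1_anim_BP to set jump, hold, throw and drop flags.
; Jump and throw flags clear after fixed delays rather than on landing or animation end.
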(event `self.CastToAnimBP_Jump`
  ;[1 1 1] Cast animation BP to jump
  (bind _asrobot_1_anim_bp (cast `/Game/Blueprints/Characters/animations_Robot1/Robot1_anim_BP` (`SkeletalMeshComponent.GetAnimInstance` (`self.Mesh`))))
  (set `/Game/Blueprints/Characters/animations_Robot1/Robot1_anim_BP.IsInAir` true _asrobot_1_anim_bp)
  (`KismetSystemLibrary.Delay` 1.0)
  (set `/Game/Blueprints/Characters/animations_Robot1/Robot1_anim_BP.IsInAir` false _asrobot_1_anim_bp))

(event `self.CastToAnimBP_Hold`
  ;[1 1 1] Cast animBP Hold
  (bind _asrobot_1_anim_bp (cast `/Game/Blueprints/Characters/animations_Robot1/Robot1_anim_BP` (`SkeletalMeshComponent.GetAnimInstance` (`self.Mesh`))))
  (set `/Game/Blueprints/Characters/animations_Robot1/Robot1_anim_BP.HoldingBall` true _asrobot_1_anim_bp))

(event `self.CastToAnimBP_Throw`
  ;[1 1 1] Cast AnimBP Throw
  (bind _asrobot_1_anim_bp (cast `/Game/Blueprints/Characters/animations_Robot1/Robot1_anim_BP` (`SkeletalMeshComponent.GetAnimInstance` (`self.Mesh`))))
  (set `/Game/Blueprints/Characters/animations_Robot1/Robot1_anim_BP.Throwing` true _asrobot_1_anim_bp)
  (set `/Game/Blueprints/Characters/animations_Robot1/Robot1_anim_BP.HoldingBall` false _asrobot_1_anim_bp)
  (`KismetSystemLibrary.Delay` 0.2)
  (set `/Game/Blueprints/Characters/animations_Robot1/Robot1_anim_BP.Throwing` false _asrobot_1_anim_bp))

(event `self.CastToAnimBP_Drop`
  ;[1 1 1] Cast to animCP Drop
  (bind _asrobot_1_anim_bp (cast `/Game/Blueprints/Characters/animations_Robot1/Robot1_anim_BP` (`SkeletalMeshComponent.GetAnimInstance` (`self.Mesh`))))
  (set `/Game/Blueprints/Characters/animations_Robot1/Robot1_anim_BP.HoldingBall` false _asrobot_1_anim_bp))

(fn `UserConstructionScript`
  (`parent.UserConstructionScript`)
  (set `self.PlayerColor` "NewEnumerator0")
  (set `self.DefaultMaterial` "/Game/Material/M_Robot1_Red.M_Robot1_Red")
  (set `self.InvulnMaterial` "/Game/Meshes/Materials/M_Red2_glow.M_Red2_glow"))