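; DodgePlayerController is a player controller that collects the PlayerStart actors assigned to its player.
; Its addToArray event scans all PlayerStarts, converts each PlayerStartTag to an integer and appends those matching its own controller ID to PlayerStarPosition.
; GetPlayerCharacter is an unfinished stub that returns nothing, with an unconnected cast to DodgeCharacter.
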(event `addToArray`
  (bind _outactors (`GameplayStatics.GetAllActorsOfClass` "/Script/Engine.PlayerStart"))
  (for _array_element _outactors
    (bind _returnvalue (`GameplayStatics.GetPlayerControllerID` self))
    (if (== _returnvalue (`KismetStringLibrary.Conv_StringToInt` (`KismetStringLibrary.Conv_NameToString` (`PlayerStart.PlayerStartTag` _array_element))))
      (`KismetArrayLibrary.Array_Add` (`self.PlayerStarPosition`) _array_element))))

(fn `GetPlayerCharacter`
  (returns (`AsThird Person Character` :type "/Game/ThirdPersonBP/Blueprints/ThirdPersonCharacter Object Reference"))
  (return null))

(fn `UserConstructionScript`)