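; Game mode for a four-player local multiplayer dodge game, handling player setup and game over.
; BeginPlay binds the game-over event, creates local players, possesses a distinct pawn class for each at hard-coded locations, and views through the shared LocalMultiplayerCamera.
; On game over, it picks the DodgePlayerController with most Points, passes its pawn to the camera, switches view to it, and replaces the score widget with the mouse-enabled game-over screen.
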(event `Find Camera Actor`
  (bind _outactors (`GameplayStatics.GetAllActorsOfClass` "/Game/Blueprints/CameraBP/LocalMultiplayerCamera.LocalMultiplayerCamera_C"))
  (set `self.MainCamera` (`|GetArrayItem` _outactors)))

(event `GameOver_Event`
  (bind _returnvalue (`GameplayStatics.GetPlayerController` 0))
  (bind _returnvalue_2 (`Controller.K2_GetPawn` (`self.WinningPlayer`)))
  (`self.GetWinningPlayer`)
  (set `/Game/Blueprints/CameraBP/LocalMultiplayerCamera.WinningPlayer` _returnvalue_2 (`self.MainCamera`))
  (`PlayerController.SetViewTargetWithBlend` _returnvalue (`self.WinCamera`) 0.0 "VTBlend_Linear" 0.0 false)
  (`PlayerController.SetViewTargetWithBlend` _returnvalue _returnvalue_2 0.0 "VTBlend_Linear" 0.0 false)
  (`GameplayStatics.SetGamePaused` false)
  (bind _returnvalue_3 (`|CreateWidget` "/Game/Blueprints/Widgets/BPW_GameOverScreen.BPW_GameOverScreen_C"))
  (`UserWidget.AddToViewport` _returnvalue_3 0)
  (`WidgetBlueprintLibrary.SetInputMode_UIOnlyEx` (`GameplayStatics.GetPlayerController` 0) (`/Game/Blueprints/Widgets/BPW_GameOverScreen.btn_playagain` _returnvalue_3))
  (set `PlayerController.bShowMouseCursor` true (`GameplayStatics.GetPlayerController` 0))
  (`Widget.RemoveFromParent` (`self.ScoreWidget`)))

(event `self.ReceiveBeginPlay`
  (`|ExecutionSequence`
    (:`then_0`
      (add `self.GameOver` (delegate `GameOver_Event`)))
    (:`then_1`
      (`self.SpawnPlayers`)
      (`self.Find Camera Actor`))
    (:`then_2`
      (`PlayerController.SetViewTargetWithBlend` (`GameplayStatics.GetPlayerController` 0) (`self.MainCamera`) 0.0 "VTBlend_Linear" 0.0 false))))

(fn `GetWinningPlayer`
  (locals (PlayerWithMostPoints :type "/Game/Blueprints/Characters/DodgePlayerController Object Reference"))
  (bind _outactors (`GameplayStatics.GetAllActorsOfClass` "/Game/Blueprints/Characters/DodgePlayerController.DodgePlayerController_C"))
  (for _array_element _outactors
    (`/Engine/EditorBlueprintResources/StandardMacros.IsValid` (`self.WinningPlayer`)
      (:`Is Valid`
        (if (> (`/Game/Blueprints/Characters/DodgePlayerController.Points` _array_element) (`/Game/Blueprints/Characters/DodgePlayerController.Points` (`self.WinningPlayer`)))
          (set `self.WinningPlayer` _array_element)))
      (:`Is Not Valid`
        (set `self.WinningPlayer` _array_element)))))

(fn `SpawnPlayers`
  (for _index (range 4)
    ;[1 1 1] add other Players
    (`GameplayStatics.CreatePlayer` _index))
  ;[1 1 1] Max antal spelare
  (for _index_2 (range 4)
    (if (== _index_2 0)
      (bind _returnvalue (`|SpawnActorFromClass` "/Game/Blueprints/Characters/ChildPlayer1.ChildPlayer1_C" (`KismetMathLibrary.MakeTransform` (322.0 -1136.0 2000.0)) "Undefined" "OverrideRootScale" null _index_2 null))
      (bind _returnvalue_2 (`GameplayStatics.GetPlayerController` _index_2))
      (`Controller.Possess` _returnvalue_2 _returnvalue)
      (elif (== _index_2 1)
        (bind _returnvalue_3 (`|SpawnActorFromClass` "/Game/Blueprints/Characters/ChildPlayer2.ChildPlayer2_C" (`KismetMathLibrary.MakeTransform` (322.0 -1136.0 900.0)) "Undefined" "OverrideRootScale" null _index_2 null))
        (`Controller.Possess` _returnvalue_2 _returnvalue_3)
        (elif (== _index_2 2)
          (bind _returnvalue_4 (`|SpawnActorFromClass` "/Game/Blueprints/Characters/ChildPlayer3.ChildPlayer3_C" (`KismetMathLibrary.MakeTransform` (322.0 -1136.0 1200.0)) "Undefined" "OverrideRootScale" null _index_2 null))
          (`Controller.Possess` _returnvalue_2 _returnvalue_4)
          (elif (== _index_2 3)
            (bind _returnvalue_5 (`|SpawnActorFromClass` "/Game/Blueprints/Characters/ChildPlayer4.ChildPlayer4_C" (`KismetMathLibrary.MakeTransform` (322.0 -1136.0 1000.0)) "Undefined" "OverrideRootScale" null _index_2 null))
            (`Controller.Possess` _returnvalue_2 _returnvalue_5)
            (else
              (`KismetSystemLibrary.PrintString` "Playerdoesn't exist"))))))))

(fn `UserConstructionScript`)